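; Blueprint function library of shared helpers, apparently for a sprite character moving along the X axis.
; Debugger conditionally prints a labeled value, and Tracer runs a Visibility line trace along X by a signed distance, returning the hit.
; SpriteRotator turns the sign of an input into an unrotated or 180-degree flipped sprite rotation plus the new direction, with zero input left unhandled.
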(fn Debugger
  (params (Condition :type Boolean) (Title :type String) (Variable :type String))
  (if Condition
    (Development|PrintString 0 (Utilities|String|Append Title Variable) true true "(R=0.000000,G=0.660000,B=1.000000,A=1.000000)" 0.0))
  (return))

(fn Tracer
  (params (WorldContextObject :type Object%20Object%20Reference) (actorLoc :type Vector) (distance :type Float%20%28single-precision%29) (direction :type Float%20%28single-precision%29) (DrawDebugType :type EDrawDebugTrace%20Enum :default "None") (DrawTime :type Float%20%28single-precision%29))
  (bind (_outhit _returnvalue) (Collision|LineTraceByChannel WorldContextObject actorLoc (+ actorLoc (Math|Vector|MakeVector (* distance direction) 0.0 0.0)) "TraceTypeQuery1" false 0 DrawDebugType true "(R=1.000000,G=0.000000,B=0.000000,A=1.000000)" "(R=0.000000,G=1.000000,B=0.000000,A=1.000000)" DrawTime))
  (return _outhit _returnvalue))

(fn SpriteRotator
  (params (f_xInput :type Float%20%28single-precision%29))
  (bind _output_get (LocalVariables|Setf_tempDir f_xInput))
  (Math|Float|CompareFloat _output_get 0.0
    (:>
      (LocalVariables|Setr_spriteRotation "0, 0, 0")
      (LocalVariables|Setf_dir (LocalVariables|Getf_tempDir)))
    (:<
      (LocalVariables|Setr_spriteRotation "0,180.000000, 0")
      (LocalVariables|Setf_dir (LocalVariables|Getf_tempDir))))
  (return (LocalVariables|Getr_spriteRotation) (LocalVariables|Getf_dir)))